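; Coliseum door actor that moves open when the third-person character enters its Box trigger carrying at least two batteries.
; BeginPlay stores the mesh's starting location, and a qualifying overlap waits briefly, then plays a Timeline lerping the mesh toward PosicionDestino.
; The graph has no closing logic, and GetInventoryData is a stub returning zero.
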(event `self.ReceiveBeginPlay`
  (set `self.PosicionInicial` (`SceneComponent.K2_GetComponentLocation` (`self.StaticMeshComponent`))))

(event `self.Box.OnComponentBeginOverlap`
  (params (OverlappedComponent :type "PrimitiveComponent Object Reference") (OtherActor :type "Actor Object Reference") (OtherComp :type "PrimitiveComponent Object Reference") (OtherBodyIndex :type Integer) (bFromSweep :type Boolean) (SweepResult :type "HitResult Structure (by ref)"))
  (bind _asbp_third_person_character (cast `/Game/ThirdPerson/Blueprints/BP_ThirdPersonCharacter` OtherActor))
  (if (>= (`/Game/ThirdPerson/Blueprints/BP_ThirdPersonCharacter.batteriesCount` _asbp_third_person_character) 2)
    (`KismetSystemLibrary.Delay` 1.0)
    (bind (_direction _alpha) (`Timeline|Timeline`)
      (:`Update`
        (`SceneComponent.K2_SetWorldLocation` (`self.StaticMeshComponent`) (`KismetMathLibrary.VLerp` (`self.PosicionInicial`) (`self.PosicionDestino`) _alpha) false false)))))

(fn `GetInventoryData`
  (returns (BatteryCount :type Integer))
  (return 0))

(fn `UserConstructionScript`)