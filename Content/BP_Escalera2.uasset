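; BP_Escalera2 is a movable mesh, named as a staircase, that a mechanism activates and deactivates.
; It caches its world location on BeginPlay, and a Timeline lerps it toward PosicionDestino without sweeping.
; Activation runs only if the PlatafomraRoja reference is valid, also making that platform's root component visible.
; Deactivation reverses the Timeline but never hides the platform again.
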(event `self.ReceiveBeginPlay`
  (set `self.PosicionInicial` (`SceneComponent.K2_GetComponentLocation` (`self.StaticMeshComponent`))))

(event `/Game/Interfaces/BPI_Mecanic.ActivarMecanismo`
  (bind _platafomraroja (`self.PlatafomraRoja`))
  (`/Engine/EditorBlueprintResources/StandardMacros.IsValid` _platafomraroja
    (:`Is Valid`
      (`SceneComponent.SetVisibility` (`Actor.RootComponent` _platafomraroja) true false)
      (bind (_direction _alpha) (`Timeline|Timeline` :!label _label)
        (:`Update`
          (`SceneComponent.K2_SetWorldLocation` (`self.StaticMeshComponent`) (`KismetMathLibrary.VLerp` (`self.PosicionInicial`) (`self.PosicionDestino`) _alpha) false false))))))

(event `/Game/Interfaces/BPI_Mecanic.DesactivarMecanismo`
  (goto _label :!via `Reverse`))

(fn `UserConstructionScript`)