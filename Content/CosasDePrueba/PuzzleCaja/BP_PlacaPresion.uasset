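; Pressure plate for a box puzzle that rewards an ability object and lowers a linked wall.
; When an actor overlaps its box trigger, an interface message checks whether it is the puzzle box.
; The first valid overlap spawns BP_ObjetoHabilidad at PuntoDeSpawn, with DoOnce blocking repeats.
; After a short delay, it calls BajarPared on ParedVinculada and plays the SequencePared level sequence.
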(event `self.Box.OnComponentBeginOverlap`
  (params (OverlappedComponent :type "PrimitiveComponent Object Reference") (OtherActor :type "Actor Object Reference") (OtherComp :type "PrimitiveComponent Object Reference") (OtherBodyIndex :type Integer) (bFromSweep :type Boolean) (SweepResult :type "HitResult Structure (by ref)"))
  (bind _esvalida (message `/Game/Interfaces/BPI_PuzzleElement.VerificarCaja` OtherActor))
  (if _esvalida
    (`/Engine/EditorBlueprintResources/StandardMacros.DoOnce` false
      (:`Completed`
        (`|SpawnActorFromClass` "/Game/CosasDePrueba/BP_ObjetoHabilidad.BP_ObjetoHabilidad_C" (`KismetMathLibrary.MakeTransform` (`SceneComponent.K2_GetComponentLocation` (`self.PuntoDeSpawn`))) "AlwaysSpawn" "MultiplyWithRoot" null null)
        (`KismetSystemLibrary.Delay` 5.0)
        (`/Game/CosasDePrueba/BP_ParedCueva.BajarPared` (`self.ParedVinculada`))
        (bind (_outactor _returnvalue) (`LevelSequencePlayer.CreateLevelSequencePlayer` (`self.SequencePared`)))
        (`MovieSceneSequencePlayer.Play` _returnvalue)))))

(fn `UserConstructionScript`)