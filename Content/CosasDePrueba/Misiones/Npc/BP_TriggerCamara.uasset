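; BP_TriggerCamara is a one-shot trigger volume that briefly cuts the player's view to an NPC map camera.
; When anything begins overlapping its Box, it disables player input and blends the view to CamaraNPCMap.
; After a five-second delay, it blends back to the player character, restores input and destroys itself.
; The overlap does not check which actor entered.
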(event `self.Box.OnComponentBeginOverlap`
  (params (OverlappedComponent :type "PrimitiveComponent Object Reference") (OtherActor :type "Actor Object Reference") (OtherComp :type "PrimitiveComponent Object Reference") (OtherBodyIndex :type Integer) (bFromSweep :type Boolean) (SweepResult :type "HitResult Structure (by ref)"))
  (bind _returnvalue (`GameplayStatics.GetPlayerController` 0))
  (bind _returnvalue_2 (`GameplayStatics.GetPlayerController` 0))
  (`self.DisableInput` (`GameplayStatics.GetPlayerCharacter` 0) _returnvalue_2)
  (`PlayerController.SetViewTargetWithBlend` _returnvalue_2 (`self.CamaraNPCMap`) 1.5 "VTBlend_Linear" 0.0 false)
  (`KismetSystemLibrary.Delay` 5.0)
  (`/Engine/EditorBlueprintResources/StandardMacros.IsValid` _returnvalue
    (:`Is Valid`
      (`PlayerController.SetViewTargetWithBlend` _returnvalue (`GameplayStatics.GetPlayerCharacter` 0) 1.5 "VTBlend_Linear" 0.0 false)
      (`self.EnableInput` (`GameplayStatics.GetPlayerCharacter` 0) (`GameplayStatics.GetPlayerController` 0))
      (`self.K2_DestroyActor`))))

(fn `UserConstructionScript`)