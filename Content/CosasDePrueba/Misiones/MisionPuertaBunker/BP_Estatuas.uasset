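; Two-statue rotation puzzle actor, in which the player turns each statue by a set yaw step with the pick-up input.
; Each statue's trigger enables input and opens a gate, and a timeline lerps the rotation while input is disabled.
; Two puzzle triggers track overlaps with BP_ActivadorEstatuas, and when both are active the actor fires the OnPuzzleResuelto dispatcher.
; Only the second statue's player trigger filters for BP_ThirdPersonCharacter.
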(event `self.ReceiveBeginPlay`
  (set `self.CurrentRotationEstatua1` (`SceneComponent.K2_GetComponentRotation` (`self.Estatua_1`)))
  (set `self.CurrentRotationEstatua2` (`SceneComponent.K2_GetComponentRotation` (`self.Estatua_2`))))

(event `EnhancedInput|/Game/Input/Actions/IA_PickUp`
  (params (ActionValue :type Boolean) (ElapsedSeconds :type "Float (double-precision)") (TriggeredSeconds :type "Float (double-precision)") (InputAction :type "InputAction Object Reference" :default "/Game/Input/Actions/IA_PickUp.IA_PickUp"))
  (:`Started`
    (`/Engine/EditorBlueprintResources/StandardMacros.Gate` true :!label _label
      (:`Exit`
        (`self.DisableInput` (`GameplayStatics.GetPlayerController` 0))
        (bind (_direction _time) (`Timeline|TimeLineEstatua1` :!via `PlayFromStart`)
          (:`Update`
            (bind _returnvalue (`KismetMathLibrary.RLerp` (`self.CurrentRotationEstatua1`) (`KismetMathLibrary.MakeRotator` (.roll (`self.CurrentRotationEstatua1`)) (.pitch (`self.CurrentRotationEstatua1`)) (+ (.yaw (`self.CurrentRotationEstatua1`)) (`self.AngleRotation`))) _time))
            (`SceneComponent.K2_SetRelativeRotation` (`self.Estatua_1`) _returnvalue false false))
          (:`Finished`
            (set `self.CurrentRotationEstatua1` _returnvalue)
            (`self.EnableInput` (`GameplayStatics.GetPlayerController` 0))))))))

(event `self.TriggerActivadorEstatua1.OnComponentBeginOverlap`
  (params (OverlappedComponent :type "PrimitiveComponent Object Reference") (OtherActor :type "Actor Object Reference") (OtherComp :type "PrimitiveComponent Object Reference") (OtherBodyIndex :type Integer) (bFromSweep :type Boolean) (SweepResult :type "HitResult Structure (by ref)"))
  (`self.EnableInput` (`GameplayStatics.GetPlayerController` 0))
  (goto _label :!via `Open`))

(event `self.TriggerActivadorEstatua1.OnComponentEndOverlap`
  (params (OverlappedComponent :type "PrimitiveComponent Object Reference") (OtherActor :type "Actor Object Reference") (OtherComp :type "PrimitiveComponent Object Reference") (OtherBodyIndex :type Integer))
  (`self.DisableInput` (`GameplayStatics.GetPlayerController` 0))
  (goto _label :!via `Close`))

(event `EnhancedInput|/Game/Input/Actions/IA_PickUp`
  (params (ActionValue :type Boolean) (ElapsedSeconds :type "Float (double-precision)") (TriggeredSeconds :type "Float (double-precision)") (InputAction :type "InputAction Object Reference" :default "/Game/Input/Actions/IA_PickUp.IA_PickUp"))
  (:`Started`
    (`/Engine/EditorBlueprintResources/StandardMacros.Gate` true :!label _label_2
      (:`Exit`
        (`self.DisableInput` (`GameplayStatics.GetPlayerController` 0))
        (bind (_direction _time) (`Timeline|Timeline` :!via `PlayFromStart`)
          (:`Update`
            (bind _returnvalue (`KismetMathLibrary.RLerp` (`self.CurrentRotationEstatua2`) (`KismetMathLibrary.MakeRotator` (.roll (`self.CurrentRotationEstatua2`)) (.pitch (`self.CurrentRotationEstatua2`)) (+ (.yaw (`self.CurrentRotationEstatua2`)) (`self.AngleRotation`))) _time))
            (`SceneComponent.K2_SetRelativeRotation` (`self.Estatua_2`) _returnvalue false false))
          (:`Finished`
            (set `self.CurrentRotationEstatua2` _returnvalue)
            (`self.EnableInput` (`GameplayStatics.GetPlayerController` 0))))))))

(event `self.TriggerActivadorEstatua2.OnComponentBeginOverlap`
  (params (OverlappedComponent :type "PrimitiveComponent Object Reference") (OtherActor :type "Actor Object Reference") (OtherComp :type "PrimitiveComponent Object Reference") (OtherBodyIndex :type Integer) (bFromSweep :type Boolean) (SweepResult :type "HitResult Structure (by ref)"))
  (cast `/Game/ThirdPerson/Blueprints/BP_ThirdPersonCharacter` OtherActor)
  (`self.EnableInput` (`GameplayStatics.GetPlayerController` 0))
  (goto _label_2 :!via `Open`))

(event `self.TriggerActivadorEstatua2.OnComponentEndOverlap`
  (params (OverlappedComponent :type "PrimitiveComponent Object Reference") (OtherActor :type "Actor Object Reference") (OtherComp :type "PrimitiveComponent Object Reference") (OtherBodyIndex :type Integer))
  (cast `/Game/ThirdPerson/Blueprints/BP_ThirdPersonCharacter` OtherActor)
  (`self.DisableInput` (`GameplayStatics.GetPlayerController` 0))
  (goto _label_2 :!via `Close`))

(event `self.TriggerActivadorPuzzle1.OnComponentBeginOverlap`
  (params (OverlappedComponent :type "PrimitiveComponent Object Reference") (OtherActor :type "Actor Object Reference") (OtherComp :type "PrimitiveComponent Object Reference") (OtherBodyIndex :type Integer) (bFromSweep :type Boolean) (SweepResult :type "HitResult Structure (by ref)"))
  (cast `/Game/CosasDePrueba/Misiones/MisionPuertaBunker/BP_ActivadorEstatuas` OtherActor)
  (bind _output_get (set `self.Estatua1Activada?` true))
  (if (and _output_get (stale `self.TriggerActivadorPuzzle2.OnComponentBeginOverlap` _output_get)) :!label _label_3
    (`self.PuzzleResuelto`)))

(event `PuzzleResuelto`
  (if (`self.Estatua1Activada?`)
    (`self.OnPuzzleResuelto`)))

(event `self.TriggerActivadorPuzzle1.OnComponentEndOverlap`
  (params (OverlappedComponent :type "PrimitiveComponent Object Reference") (OtherActor :type "Actor Object Reference") (OtherComp :type "PrimitiveComponent Object Reference") (OtherBodyIndex :type Integer))
  (cast `/Game/CosasDePrueba/Misiones/MisionPuertaBunker/BP_ActivadorEstatuas` OtherActor)
  (set `self.Estatua1Activada?` false))

(event `self.TriggerActivadorPuzzle2.OnComponentBeginOverlap`
  (params (OverlappedComponent :type "PrimitiveComponent Object Reference") (OtherActor :type "Actor Object Reference") (OtherComp :type "PrimitiveComponent Object Reference") (OtherBodyIndex :type Integer) (bFromSweep :type Boolean) (SweepResult :type "HitResult Structure (by ref)"))
  (cast `/Game/CosasDePrueba/Misiones/MisionPuertaBunker/BP_ActivadorEstatuas` OtherActor)
  (bind _output_get (set `self.Estatua2Activada?` true))
  (goto _label_3))

(event `self.TriggerActivadorPuzzle2.OnComponentEndOverlap`
  (params (OverlappedComponent :type "PrimitiveComponent Object Reference") (OtherActor :type "Actor Object Reference") (OtherComp :type "PrimitiveComponent Object Reference") (OtherBodyIndex :type Integer))
  (cast `/Game/CosasDePrueba/Misiones/MisionPuertaBunker/BP_ActivadorEstatuas` OtherActor)
  (set `self.Estatua2Activada?` false))

(fn `UserConstructionScript`)