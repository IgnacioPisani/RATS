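; BP_Elevador is a one-shot elevator that raises its cube platform in a short camera-driven sequence.
; A box overlap asks the entering actor through PreguntarTieneControlMessage and, if true, triggers once after a brief delay.
; Player input is disabled and the view blends to the elevator while the Anim_Subir timeline lerps the cube from its starting position to PosicionDestino.
; On completion, input and player view are restored.
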(event `self.ReceiveBeginPlay`
  (set `self.PosicionInicial` (`SceneComponent.K2_GetComponentLocation` (`self.Cube`))))

(event `self.Box.OnComponentBeginOverlap`
  (params (OverlappedComponent :type "PrimitiveComponent Object Reference") (OtherActor :type "Actor Object Reference") (OtherComp :type "PrimitiveComponent Object Reference") (OtherBodyIndex :type Integer) (bFromSweep :type Boolean) (SweepResult :type "HitResult Structure (by ref)"))
  (bind _returnvalue (`GameplayStatics.GetPlayerCharacter` 0))
  (bind _returnvalue_2 (`PlayerState.GetPlayerController` (`Pawn.PlayerState` _returnvalue)))
  (bind _btiene (message `/Game/CosasDePrueba/Misiones/TorreElevador/BPI_ChecksJugador.Preguntar_TieneControl` OtherActor))
  (if _btiene
    (`/Engine/EditorBlueprintResources/StandardMacros.DoOnce` false
      (:`Completed`
        (`KismetSystemLibrary.Delay` 2.0)
        (`self.DisableInput` _returnvalue _returnvalue_2)
        (`PlayerController.SetViewTargetWithBlend` _returnvalue_2 self 2.0 "VTBlend_Cubic" 0.0 false)
        (bind (_direction _alpha) (`Timeline|Anim_Subir`)
          (:`Update`
            (`SceneComponent.K2_SetWorldLocation` (`self.Cube`) (`KismetMathLibrary.VLerp` (`self.PosicionInicial`) (`self.PosicionDestino`) _alpha) false false))
          (:`Finished`
            (`self.EnableInput` _returnvalue _returnvalue_2)
            (`PlayerController.SetViewTargetWithBlend` (`GameplayStatics.GetPlayerController` 0) (`GameplayStatics.GetPlayerCharacter` 0) 1.5 "VTBlend_Linear" 0.0 false)))))))

(fn `UserConstructionScript`)