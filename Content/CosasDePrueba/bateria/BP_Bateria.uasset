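; BP_Bateria is a battery actor that plays a one-time cutscene when its trigger box is overlapped.
; After a short delay, it disables player input and starts the LS_Bateria level sequence.
; Alongside it, the Anim_Subir timeline lerps the battery from its starting position to PosicionDestino, then restores input and destroys the actor.
; The overlap does not check which actor entered.
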(event `self.ReceiveBeginPlay`
  (set `self.PosicionInicial` (`SceneComponent.K2_GetComponentLocation` (`self.bateria`))))

(event `self.Box.OnComponentBeginOverlap`
  (params (OverlappedComponent :type "PrimitiveComponent Object Reference") (OtherActor :type "Actor Object Reference") (OtherComp :type "PrimitiveComponent Object Reference") (OtherBodyIndex :type Integer) (bFromSweep :type Boolean) (SweepResult :type "HitResult Structure (by ref)"))
  (bind _returnvalue (`GameplayStatics.GetPlayerCharacter` 0))
  (bind _returnvalue_2 (`GameplayStatics.GetPlayerCharacter` 0))
  (`/Engine/EditorBlueprintResources/StandardMacros.DoOnce` false
    (:`Completed`
      (`KismetSystemLibrary.Delay` 2.0)
      (`self.DisableInput` _returnvalue_2 (`PlayerState.GetPlayerController` (`Pawn.PlayerState` _returnvalue_2)))
      (bind (_outactor _returnvalue_3) (`LevelSequencePlayer.CreateLevelSequencePlayer` "/Game/CosasDePrueba/bateria/LS_Bateria.LS_Bateria"))
      (`MovieSceneSequencePlayer.Play` _returnvalue_3)
      (bind (_direction _alpha) (`Timeline|Anim_Subir`)
        (:`Update`
          (`SceneComponent.K2_SetWorldLocation` (`self.bateria`) (`KismetMathLibrary.VLerp` (`self.PosicionInicial`) (`self.PosicionDestino`) _alpha) false false))
        (:`Finished`
          (`self.EnableInput` _returnvalue (`PlayerState.GetPlayerController` (`Pawn.PlayerState` _returnvalue)))
          (`self.K2_DestroyActor`))))))

(fn `UserConstructionScript`)