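; BP_IslaFlotanteM is a floating island that travels one way to a destination once a qualifying actor enters its trigger box.
; An overlap asks the actor through PreguntarTieneControlMessage whether it has control; the first positive answer passes a DoOnce and starts a short delay.
; A Timeline then lerps the static mesh's world location, without sweep, from the position cached at BeginPlay to PosicionDestino.
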(event `self.ReceiveBeginPlay`
  (set `self.PosicionInicial` (`SceneComponent.K2_GetComponentLocation` (`self.StaticMesh`))))

(event `self.Box.OnComponentBeginOverlap`
  (params (OverlappedComponent :type "PrimitiveComponent Object Reference") (OtherActor :type "Actor Object Reference") (OtherComp :type "PrimitiveComponent Object Reference") (OtherBodyIndex :type Integer) (bFromSweep :type Boolean) (SweepResult :type "HitResult Structure (by ref)"))
  (bind _btiene (message `/Game/CosasDePrueba/Misiones/TorreElevador/BPI_ChecksJugador.Preguntar_TieneControl` OtherActor))
  (if _btiene
    (`/Engine/EditorBlueprintResources/StandardMacros.DoOnce` false
      (:`Completed`
        (`KismetSystemLibrary.Delay` 2.0)
        (bind (_direction _alpha) (`Timeline|Timeline`)
          (:`Update`
            (`SceneComponent.K2_SetWorldLocation` (`self.StaticMesh`) (`KismetMathLibrary.VLerp` (`self.PosicionInicial`) (`self.PosicionDestino`) _alpha) false false)))))))

(fn `UserConstructionScript`)