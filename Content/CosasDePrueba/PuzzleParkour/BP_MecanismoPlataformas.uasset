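; BP_MecanismoPlataformas is a parkour puzzle mechanism that reveals a list of platforms one after another.
; ActivarMecanismo starts AparecerEnCadena, which unhides and enables collision on the current platform in ListaDePlataformas.
; The event then increments IndiceAparicion, waits a short delay and calls itself until the list ends.
; DesactivarMecanismo is an empty stub, and the index is never reset here.
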(event `AparecerEnCadena`
  (bind _indiceaparicion (`self.IndiceAparicion`))
  (bind _listadeplataformas (`self.ListaDePlataformas`))
  (bind _output (`|GetArrayItem` _listadeplataformas _indiceaparicion))
  (if (< _indiceaparicion (`KismetArrayLibrary.Array_Length` _listadeplataformas))
    (`self.SetActorHiddenInGame` _output false)
    (`self.SetActorEnableCollision` _output true)
    (`/Engine/EditorBlueprintResources/StandardMacros.IncrementInt` (`self.IndiceAparicion`)
      (:`  `
        (`KismetSystemLibrary.Delay` 0.5)
        (`self.AparecerEnCadena`)))))

(event `/Game/Interfaces/BPI_Mecanic.ActivarMecanismo`
  (`self.AparecerEnCadena`))

(event `/Game/Interfaces/BPI_Mecanic.DesactivarMecanismo`)

(fn `UserConstructionScript`)