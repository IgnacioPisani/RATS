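; Elevator Blueprint that lifts a platform once and then plays a tower panning cinematic.
; When an overlapping actor answers that it has control, a DoOnce starts a delayed timeline that lerps the cube from its initial location to a destination.
; Player input is disabled during the ride, restored on arrival, then disabled again after a pause while the EQ_PaneoTorre level sequence plays, and re-enabled when it finishes.
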(event `self.ReceiveBeginPlay`
  (set `self.PosicionInicial` (`SceneComponent.K2_GetComponentLocation` (`self.Cube`))))

(event `self.Box.OnComponentBeginOverlap`
  (params (OverlappedComponent :type "PrimitiveComponent Object Reference") (OtherActor :type "Actor Object Reference") (OtherComp :type "PrimitiveComponent Object Reference") (OtherBodyIndex :type Integer) (bFromSweep :type Boolean) (SweepResult :type "HitResult Structure (by ref)"))
  (bind _returnvalue (`GameplayStatics.GetPlayerCharacter` 0))
  (bind _returnvalue_2 (`GameplayStatics.GetPlayerCharacter` 0))
  (bind _returnvalue_3 (`PlayerState.GetPlayerController` (`Pawn.PlayerState` _returnvalue)))
  (bind _btiene (message `/Game/CosasDePrueba/TorreElevador/BPI_ChecksJugador.Preguntar_TieneControl` OtherActor))
  (`KismetSystemLibrary.PrintString` (`KismetStringLibrary.Conv_BoolToString` _btiene))
  (if _btiene
    (`/Engine/EditorBlueprintResources/StandardMacros.DoOnce` false
      (:`Completed`
        (`KismetSystemLibrary.Delay` 2.0)
        (`self.DisableInput` _returnvalue_2 (`PlayerState.GetPlayerController` (`Pawn.PlayerState` _returnvalue_2)))
        (bind (_direction _alpha) (`Timeline|Anim_Subir`)
          (:`Update`
            (`SceneComponent.K2_SetWorldLocation` (`self.Cube`) (`KismetMathLibrary.VLerp` (`self.PosicionInicial`) (`self.PosicionDestino`) _alpha) false false))
          (:`Finished`
            (`self.EnableInput` _returnvalue _returnvalue_3)
            (`KismetSystemLibrary.Delay` 5.0)
            (`self.DisableInput` _returnvalue _returnvalue_3)
            (bind (_outactor _returnvalue_4) (`LevelSequencePlayer.CreateLevelSequencePlayer` "/Game/CosasDePrueba/EQ_PaneoTorre.EQ_PaneoTorre"))
            (`MovieSceneSequencePlayer.Play` _returnvalue_4)
            (add `MovieSceneSequencePlayer.OnFinished` _returnvalue_4 (delegate `AlTerminarPaneo`))))))))

(event `AlTerminarPaneo`
  (bind _returnvalue (`GameplayStatics.GetPlayerCharacter` 0))
  (`self.EnableInput` _returnvalue (`PlayerState.GetPlayerController` (`Pawn.PlayerState` _returnvalue))))

(fn `UserConstructionScript`)