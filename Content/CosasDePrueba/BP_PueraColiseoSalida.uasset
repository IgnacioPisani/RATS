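; Coliseum exit door actor that opens after a boss is defeated by moving its static mesh.
; It records the mesh's starting world location on BeginPlay.
; OnBossDefeated waits a few seconds, plays a door level sequence, and runs a Timeline that lerps the mesh to PosicionDestino without sweep.
; GetInventoryData is a stub that returns zero.
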(event `self.ReceiveBeginPlay`
  (set `self.PosicionInicial` (`SceneComponent.K2_GetComponentLocation` (`self.StaticMeshComponent`))))

(event `/Game/Interfaces/BPI_BossEvents.OnBossDefeated`
  (`KismetSystemLibrary.Delay` 6.0)
  (bind (_outactor _returnvalue) (`LevelSequencePlayer.CreateLevelSequencePlayer` (`self.SequencePuerta`)))
  (`MovieSceneSequencePlayer.Play` _returnvalue)
  (bind (_direction _alpha) (`Timeline|Timeline`)
    (:`Update`
      (`SceneComponent.K2_SetWorldLocation` (`self.StaticMeshComponent`) (`KismetMathLibrary.VLerp` (`self.PosicionInicial`) (`self.PosicionDestino`) _alpha) false false))))

(fn `GetInventoryData`
  (returns (BatteryCount :type Integer))
  (return 0))

(fn `UserConstructionScript`)