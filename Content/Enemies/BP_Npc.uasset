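; BP_Npc is an NPC that loops a broken-robot animation and delivers a mission-complete dialogue when approached.
; An InteractionSphere overlap queries the other actor through BPI_PlayerInventory and proceeds only when its inventory data message matches the expected value.
; It then creates a dialogue widget, feeds it the FilaMisionCumplida row from DT_Dialogue_Npc1, and removes it after a short delay.
; GetItemData is an empty stub.
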(event `self.ReceiveBeginPlay`
  (`SkeletalMeshComponent.PlayAnimation` (`self.Mesh`) "/Game/Arbol/AnimacionPorfinRobotHeladera3_Anim_Armadura_RobotRoto.AnimacionPorfinRobotHeladera3_Anim_Armadura_RobotRoto" true))

(event `self.InteractionSphere.OnComponentBeginOverlap`
  (params (OverlappedComponent :type "PrimitiveComponent Object Reference") (OtherActor :type "Actor Object Reference") (OtherComp :type "PrimitiveComponent Object Reference") (OtherBodyIndex :type Integer) (bFromSweep :type Boolean) (SweepResult :type "HitResult Structure (by ref)"))
  (if (`KismetSystemLibrary.DoesImplementInterface` OtherActor "/Game/Interfaces/BPI_PlayerInventory.BPI_PlayerInventory_C")
    (bind _batterycount (message `/Game/Interfaces/BPI_PlayerInventory.GetInventoryData` OtherActor))
    (if (== _batterycount 2)
      (bind _returnvalue (`|CreateWidget` "/Game/Widget/WBP_DialogueWidget.WBP_DialogueWidget_C"))
      (bind _output_get (set `self.WidgetDeDialogoActivo` _returnvalue))
      (`UserWidget.AddToViewport` _output_get 0)
      (bind _returnvalue_2 (`|GetDataTableRow` "/Game/DT_Dialogue_Npc1.DT_Dialogue_Npc1" (`self.FilaMisionCumplida`))
        (:`then`
          (`DialogueWidget.StartDialogueLine` (`self.WidgetDeDialogoActivo`) _returnvalue_2)
          (`KismetSystemLibrary.Delay` 5.0)
          (`Widget.RemoveFromParent` (`self.WidgetDeDialogoActivo`)))))))

(fn `GetItemData`
  (returns (ItemData :type "/Game/ThirdPerson/Blueprints/S_ItemStruct Structure"))
  (return))

(fn `UserConstructionScript`)