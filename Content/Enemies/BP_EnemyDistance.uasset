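; Ranged ("Distance") enemy that mirrors a target-reached flag to the blackboard of its IA_EnemyDistance controller and spawns Niagara damage effects at impact points.
; BeginPlay sets the flag true, while SetEnemyLocation stores a destination, marks the enemy moving and clears it.
; Tick's movement branch is empty: two movement attempts with arrival checks are disconnected, so nothing here moves the enemy or sets the flag true again.
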(event `self.ReceiveBeginPlay`
  (set `self.HasReachedTarget?` true)
  (bind _asia_enemy_distance (cast `/Game/Enemies/IA/IA_EnemyDistance` (`self.GetController`)))
  (`BlackboardComponent.SetValueAsBool` (`AIBlueprintHelperLibrary.GetBlackboard` _asia_enemy_distance) (`self.KeyName`) (`self.HasReachedTarget?`)))

(event `self.ReceivedDamage`
  (params (Damage :type "Float (single-precision)") (ImpactPoint :type "Vector Structure (by ref)") (DamageDirection :type "Vector Structure (by ref)"))
  (`NiagaraFunctionLibrary.SpawnSystemAtLocation` "/Game/Variant_Combat/VFX/NS_Damage.NS_Damage" ImpactPoint (`KismetMathLibrary.Conv_VectorToRotator` DamageDirection)))

(event `self.ReceiveTick`
  (params (DeltaSeconds :type "Float (single-precision)"))
  (if (`self.IsMoving?`)
    _))

(fn `SetEnemyLocation`
  (params (NewLocation :type "Vector Structure"))
  (returns (Result :type Boolean))
  (set `self.LocationToMove` NewLocation)
  (set `self.IsMoving?` true)
  (set `self.HasReachedTarget?` false)
  (bind _asia_enemy_distance (cast `/Game/Enemies/IA/IA_EnemyDistance` (`self.GetController`)))
  (`BlackboardComponent.SetValueAsBool` (`AIBlueprintHelperLibrary.GetBlackboard` _asia_enemy_distance) (`self.KeyName`) (`self.HasReachedTarget?`))
  (return true))

(fn `UserConstructionScript`)