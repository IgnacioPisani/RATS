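; Enemy Blueprint that performs a melee combo attack against the third-person player character.
; Attack plays the combo montage on the mesh, using IsAttacking to block retriggering until it completes or is interrupted.
; HandleHit sphere-traces for pawns from the right-hand socket along a fixed world-forward vector, since its rotation input is zero, and applies damage to a hit BP_ThirdPersonCharacter.
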(event `/Game/Enemies/BPI_Attack.Attack`
  (if (not (`self.bIsAttacking?`))
    (`|PlayMontage` (`self.Mesh`) "/Game/Variant_Combat/Anims/AM_ComboAttack.AM_ComboAttack"
      (:`then`
        (set `self.bIsAttacking?` true))
      (:`OnCompleted`
        (set `self.bIsAttacking?` false :!label _label))
      (:`OnInterrupted`
        (goto _label)))))

(event `/Game/Enemies/BPI_HandleHit.HandleHit`
  (bind _returnvalue (`SceneComponent.GetSocketLocation` (`self.Mesh`) "hand_rSocket"))
  (bind _outhit (`KismetSystemLibrary.SphereTraceSingleForObjects` _returnvalue (+ _returnvalue (* (`KismetMathLibrary.GetForwardVector` (struct)) 50.0)) 10.0 (`|MakeArray` "ObjectTypeQuery3" :!type "EObjectTypeQuery Enum")))
  (bind _asbp_third_person_character (cast `/Game/ThirdPerson/Blueprints/BP_ThirdPersonCharacter` (`.HitActor` (`GameplayStatics.BreakHitResult` _outhit))))
  (`GameplayStatics.ApplyDamage` _asbp_third_person_character 10.0 null self))

(fn `UserConstructionScript`)