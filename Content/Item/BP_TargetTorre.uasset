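; BP_TargetTorre is a tower target that moves a linked elevator (Elevador) when destroyed.
; BeginPlay caches the elevator's location and a second point 3720 units above it.
; DestroyTarget runs once, playing a timeline whose ElevadorBajarTrack blends the elevator from the raised point (alpha 0) to the original (alpha 1).
; DestroyActor is wired to the timeline's Update, so the target destroys itself on the first update.
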(event `self.ReceiveBeginPlay`
  (bind _output_get (set `self.PosicionInicialTorre` (`SceneComponent.K2_GetComponentLocation` (`Actor.RootComponent` (`self.Elevador`)))))
  (set `self.PosicionFinalTorre` (- _output_get (0.0 0.0 -3720.0))))

(event `/Game/Interfaces/BPI_DestroyTarget.DestroyTarget`
  (`/Engine/EditorBlueprintResources/StandardMacros.DoOnce` false
    (:`Completed`
      (bind (_direction _elevadorbajartrack) (`Timeline|Timeline`)
        (:`Update`
          (`SceneComponent.K2_SetWorldLocation` (`Actor.RootComponent` (`self.Elevador`)) (`KismetMathLibrary.VLerp` (`self.PosicionFinalTorre`) (`self.PosicionInicialTorre`) _elevadorbajartrack) false false)
          (`self.K2_DestroyActor`))))))

(fn `UserConstructionScript`)