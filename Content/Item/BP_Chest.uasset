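; BP_Chest is an interactable loot chest that opens once and releases the item held in its SpawnItemData.
; The first Interact plays the opening animation, shows a point light and Niagara effect, and spawns a BP_ItemIcon at a world-space offset from the chest with that item data.
; It then clears the stored item and, after a short delay, EndLoot hides the light and effect.
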(event `self.ReceiveBeginPlay`
  (set `self.ItemData` (make `ItemStruct` "Chest")))

(event `self.Interact`
  (params (Interactor :type "Actor Object Reference"))
  (bind _returnvalue (`self.GetTransform`))
  (bind (_spawnitemdata_name _spawnitemdata_bstackable _spawnitemdata_quantity _spawnitemdata_thumbnail _spawnitemdata_mesh) (break `ItemStruct` (`self.SpawnItemData`)))
  (set `self.SpawnItemData` (make `ItemStruct` _spawnitemdata_name _spawnitemdata_bstackable 0 _spawnitemdata_thumbnail _spawnitemdata_mesh))
  (if (not (`self.bIsActivated`))
    (`SkeletalMeshComponent.PlayAnimation` (`self.SkeletalMesh`) "/Game/Item/Cofrev12_Anim.Cofrev12_Anim" false)
    (set `self.bIsActivated` true)
    (`SceneComponent.SetVisibility` (`self.PointLight`) true false)
    (`SceneComponent.SetVisibility` (`self.Niagara`) true false)
    (`|SpawnActorFromClass` "/Game/Item/BP_ItemIcon.BP_ItemIcon_C" (`KismetMathLibrary.MakeTransform` (`KismetMathLibrary.MakeVector` (.x (.location _returnvalue)) (+ (.y (.location _returnvalue)) 100.0) (+ (.z (.location _returnvalue)) 200.0)) (struct) (.scale _returnvalue)) "Undefined" "MultiplyWithRoot" null (`self.SpawnItemData`) null)
    (set `self.SpawnItemData` (make `ItemStruct` "None"))
    (`KismetSystemLibrary.Delay` 2.0)
    (`self.EndLoot`)))

(fn `EndLoot`
  (`SceneComponent.SetVisibility` (`self.PointLight`) false false)
  (`SceneComponent.SetVisibility` (`self.Niagara`) false false))

(fn `UserConstructionScript`
  (set `self.ItemData` (make `ItemStruct` "Chest")))