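; BP_Item is an item actor with a static mesh that behaves differently when it comes from a chest.
; If IsFromChest is set, BeginPlay turns off physics simulation and gravity on the mesh.
; Tick then spins the actor steadily around its yaw axis, scaled by delta time.
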(event `self.ReceiveBeginPlay`
  (if (`self.isFromChest?`)
    (`PrimitiveComponent.SetSimulatePhysics` (`self.StaticMesh`) false)
    (`PrimitiveComponent.SetEnableGravity` (`self.StaticMesh`) false)))

(event `self.ReceiveTick`
  (params (DeltaSeconds :type "Float (single-precision)"))
  (if (`self.isFromChest?`)
    (`self.K2_AddActorLocalRotation` (`KismetMathLibrary.MakeRotator` 0.0 0.0 (* DeltaSeconds 300.0)))))

(fn `UserConstructionScript`)