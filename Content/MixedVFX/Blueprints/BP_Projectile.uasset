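; BP_Projectile is a projectile actor that shows a selectable Niagara effect and damages whatever it hits.
; On BeginPlay it casts the player pawn to BP_MainCamera and sets its Niagara component's asset from that camera's template array, using the clamped current effect index.
; When its Box component registers a hit, it applies fixed damage to the hit actor and destroys itself.
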(event `self.ReceiveBeginPlay`
  (bind _asbp_main_camera (cast `/Game/MixedVFX/Blueprints/BP_MainCamera` (`GameplayStatics.GetPlayerPawn` 0)))
  (`NiagaraComponent.SetAsset` (`self.Niagara`) (`|GetArrayItem` (`/Game/MixedVFX/Blueprints/BP_MainCamera.NiagaraTemplate` _asbp_main_camera) (`KismetMathLibrary.Clamp` (`/Game/MixedVFX/Blueprints/BP_MainCamera.NiagaraID` _asbp_main_camera) 0 20)) true))

(event `self.Box.OnComponentHit`
  (params (HitComponent :type "PrimitiveComponent Object Reference") (OtherActor :type "Actor Object Reference") (OtherComp :type "PrimitiveComponent Object Reference") (NormalImpulse :type "Vector Structure") (Hit :type "HitResult Structure (by ref)"))
  (`GameplayStatics.ApplyDamage` (`.HitActor` (`GameplayStatics.BreakHitResult` Hit)) 30.0)
  (`self.K2_DestroyActor`))

(fn `UserConstructionScript`)