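; Parkour platform actor that moves its mesh along a spline when the player presses the pick-up input near it.
; A box overlap enables input for player 0 and disables it on exit, without checking which actor overlaps.
; The input waits a short delay, then plays a Timeline that maps alpha to spline distance and sets the mesh's world transform, with no reverse.
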(event `EnhancedInput|/Game/Input/Actions/IA_PickUp`
  (params (ActionValue :type Boolean) (ElapsedSeconds :type "Float (double-precision)") (TriggeredSeconds :type "Float (double-precision)") (InputAction :type "InputAction Object Reference" :default "/Game/Input/Actions/IA_PickUp.IA_PickUp"))
  (bind _spline (`self.Spline`))
  (:`Started`
    (`KismetSystemLibrary.Delay` 1.0)
    (bind (_direction _alpha) (`Timeline|Timeline`)
      (:`Update`
        (`SceneComponent.K2_SetWorldTransform` (`self.StaticMesh1`) (`SplineComponent.GetTransformAtDistanceAlongSpline` _spline (* (`SplineComponent.GetSplineLength` _spline) _alpha) "World" false) false false)))))

(event `self.Box.OnComponentBeginOverlap`
  (params (OverlappedComponent :type "PrimitiveComponent Object Reference") (OtherActor :type "Actor Object Reference") (OtherComp :type "PrimitiveComponent Object Reference") (OtherBodyIndex :type Integer) (bFromSweep :type Boolean) (SweepResult :type "HitResult Structure (by ref)"))
  (`self.EnableInput` (`GameplayStatics.GetPlayerController` 0)))

(event `self.Box.OnComponentEndOverlap`
  (params (OverlappedComponent :type "PrimitiveComponent Object Reference") (OtherActor :type "Actor Object Reference") (OtherComp :type "PrimitiveComponent Object Reference") (OtherBodyIndex :type Integer))
  (`self.DisableInput` (`GameplayStatics.GetPlayerController` 0)))

(fn `UserConstructionScript`)