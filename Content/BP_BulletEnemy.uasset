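; BP_BulletEnemy is an enemy bullet actor that flies from a start location toward a target location and damages what it overlaps.
; On BeginPlay it sets its lifespan from VisualDuration, then aims the ProjectileMovement velocity and actor rotation along that line at a fixed speed.
; A distance-over-duration speed is computed, but the movement uses the hardcoded value instead.
; Sphere overlap applies fixed damage without destroying the bullet.
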(event `self.ReceiveBeginPlay`
  (bind _targetlocation (`self.TargetLocation`))
  (bind _startlocation (`self.StartLocation`))
  (bind _projectilemovement (`self.ProjectileMovement`))
  (`self.SetLifeSpan` (`self.VisualDuration`))
  (if (<= (`self.VisualDuration`) 0.01)
    (set `self.VisualDuration` 0.1))
  (set `self.InitialSpeed` (/ (`KismetMathLibrary.Vector_Distance` (`self.TargetLocation`) (`self.StartLocation`)) (`self.VisualDuration`)))
  (set `ProjectileMovementComponent.InitialSpeed` 18000.0 _projectilemovement)
  (set `ProjectileMovementComponent.MaxSpeed` 18000.0 _projectilemovement)
  (set `MovementComponent.Velocity` (* (`KismetMathLibrary.Normal` (- _targetlocation _startlocation)) (`ProjectileMovementComponent.InitialSpeed` _projectilemovement)) (`self.ProjectileMovement`))
  (`self.K2_SetActorRotation` (`KismetMathLibrary.FindLookAtRotation` _startlocation _targetlocation)))

(event `self.Sphere.OnComponentBeginOverlap`
  (params (OverlappedComponent :type "PrimitiveComponent Object Reference") (OtherActor :type "Actor Object Reference") (OtherComp :type "PrimitiveComponent Object Reference") (OtherBodyIndex :type Integer) (bFromSweep :type Boolean) (SweepResult :type "HitResult Structure (by ref)"))
  (`GameplayStatics.ApplyDamage` OtherActor 15.0))

(fn `UserConstructionScript`)