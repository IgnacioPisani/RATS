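; BP_EnemyMelee2 is a melee enemy that starts an AI move toward the player character on BeginPlay.
; Each tick it rotates its health bar widget to face the player camera.
; Attack plays a scorpion attack montage, guarded by an IsAttacking flag that clears when the montage completes or is interrupted.
; A damage event spawns a Niagara hit effect at the impact point, oriented along the damage direction.
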(event `self.ReceiveBeginPlay`
  (`|AIMoveTo` self (0.0 0.0 0.0) (`GameplayStatics.GetPlayerCharacter` 0)))

(event `self.ReceiveTick`
  (params (DeltaSeconds :type "Float (single-precision)"))
  (bind _healthbarwidgetcomponent (`self.HealthBarWidgetComponent`))
  (`SceneComponent.K2_SetWorldRotation` _healthbarwidgetcomponent (`KismetMathLibrary.FindLookAtRotation` (`SceneComponent.K2_GetComponentLocation` _healthbarwidgetcomponent) (`SceneComponent.K2_GetComponentLocation` (`PlayerCameraManager.TransformComponent` (`GameplayStatics.GetPlayerCameraManager` 0)))) false false))

(event `self.Attack`
  (if (not (`self.bIsAttacking?`))
    (`|PlayMontage` (`self.Mesh`) "/Game/Enemies/Escorpion/Scorpion_Anim_Armature_Attack_Montage.Scorpion_Anim_Armature_Attack_Montage"
      (:`then`
        (set `self.bIsAttacking?` true))
      (:`OnCompleted`
        (set `self.bIsAttacking?` false :!label _label))
      (:`OnInterrupted`
        (goto _label)))))

(event `self.ReceivedDamage`
  (params (Damage :type "Float (single-precision)") (ImpactPoint :type "Vector Structure (by ref)") (DamageDirection :type "Vector Structure (by ref)"))
  (`NiagaraFunctionLibrary.SpawnSystemAtLocation` "/Game/Variant_Combat/VFX/NS_Damage.NS_Damage" ImpactPoint (`KismetMathLibrary.Conv_VectorToRotator` DamageDirection)))

(fn `UserConstructionScript`)