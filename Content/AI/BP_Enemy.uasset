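; Enemy AI that roams between random tagged actors, chases the player character when perceived, and damages actors that overlap its capsule.
; Patrol loops through AIMoveTo, pausing briefly after each successful arrival.
; Any AIPerception update on BP_ThirdPersonCharacter raises walk speed and moves toward it, without checking whether sensing succeeded.
; Forgetting that character lowers speed and re-enters the patrol loop.
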(event `self.ReceiveBeginPlay`
  (add `AIPerceptionComponent.OnTargetPerceptionForgotten` (`self.AIPerception`) (delegate `OnTargetPerceptionForgotten_Event`))
  (bind _outactors (`GameplayStatics.GetAllActorsWithTag` (`self.Tag`) :!label _label))
  (`|AIMoveTo` self (0.0 0.0 0.0) (`KismetArrayLibrary.Array_Random` _outactors) 0.0
    (:`OnSuccess`
      (`KismetSystemLibrary.Delay` 2.0)
      (goto _label))))

(event `OnTargetPerceptionForgotten_Event`
  (params (Actor :type "Actor Object Reference")))

(event `self.AIPerception.OnTargetPerceptionForgotten`
  (params (Actor :type "Actor Object Reference"))
  (cast `/Game/ThirdPerson/Blueprints/BP_ThirdPersonCharacter` Actor)
  (set `CharacterMovementComponent.MaxWalkSpeed` 300.0 (`self.CharacterMovement`))
  (goto _label))

(event `self.AIPerception.OnTargetPerceptionUpdated`
  (params (Actor :type "Actor Object Reference") (Stimulus :type "AIStimulus Structure"))
  (bind _asbp_third_person_character (cast `/Game/ThirdPerson/Blueprints/BP_ThirdPersonCharacter` Actor))
  (set `CharacterMovementComponent.MaxWalkSpeed` 500.0 (`self.CharacterMovement`))
  (`|AIMoveTo` self (0.0 0.0 0.0) _asbp_third_person_character))

(event `self.CapsuleComponent.OnComponentBeginOverlap`
  (params (OverlappedComponent :type "PrimitiveComponent Object Reference") (OtherActor :type "Actor Object Reference") (OtherComp :type "PrimitiveComponent Object Reference") (OtherBodyIndex :type Integer) (bFromSweep :type Boolean) (SweepResult :type "HitResult Structure (by ref)"))
  (`GameplayStatics.ApplyDamage` OtherActor 30.0 null self))

(fn `UserConstructionScript`)