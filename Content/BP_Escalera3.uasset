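; BP_Escalera3 is a staircase or ladder actor whose static mesh rotates when its mechanism is activated or deactivated.
; BeginPlay stores the mesh's starting world rotation as RotacionInicial.
; ActivarMecanismo plays a timeline that lerps the mesh from that rotation toward RotacionDestino, and DesactivarMecanismo reverses the same timeline to return it.
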(event `self.ReceiveBeginPlay`
  (set `self.RotacionInicial` (`SceneComponent.K2_GetComponentRotation` (`self.StaticMeshComponent`))))

(event `/Game/Interfaces/BPI_Mecanic.ActivarMecanismo`
  (bind (_direction _alpha) (`Timeline|Timeline` :!label _label)
    (:`Update`
      (`SceneComponent.K2_SetWorldRotation` (`self.StaticMeshComponent`) (`KismetMathLibrary.RLerp` (`self.RotacionInicial`) (`self.RotacionDestino`) _alpha) false false))))

(event `/Game/Interfaces/BPI_Mecanic.DesactivarMecanismo`
  (goto _label :!via `Reverse`))

(fn `UserConstructionScript`)