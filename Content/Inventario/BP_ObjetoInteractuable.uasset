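; BP_ObjetoInteractuable is an interactable world item that can load its item data into the player's inventory.
; Its Box overlap events set and clear the ObjetoInteractuable reference on BP_ThirdPersonCharacter.
; Interactuar asks the player's Inventario for space via ComprobarHueco and, if there is room, passes DatosObjeto to CargarObjeto at the returned position.
; The actor stays in the world afterwards, as nothing here destroys or hides it.
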(event `self.Box.OnComponentBeginOverlap`
  (params (OverlappedComponent :type "PrimitiveComponent Object Reference") (OtherActor :type "Actor Object Reference") (OtherComp :type "PrimitiveComponent Object Reference") (OtherBodyIndex :type Integer) (bFromSweep :type Boolean) (SweepResult :type "HitResult Structure (by ref)"))
  (bind _asbp_third_person_character (cast `/Game/ThirdPerson/Blueprints/BP_ThirdPersonCharacter` OtherActor))
  (set `/Game/ThirdPerson/Blueprints/BP_ThirdPersonCharacter.ObjetoInteractuable` self _asbp_third_person_character))

(event `self.Box.OnComponentEndOverlap`
  (params (OverlappedComponent :type "PrimitiveComponent Object Reference") (OtherActor :type "Actor Object Reference") (OtherComp :type "PrimitiveComponent Object Reference") (OtherBodyIndex :type Integer))
  (bind _asbp_third_person_character (cast `/Game/ThirdPerson/Blueprints/BP_ThirdPersonCharacter` OtherActor))
  (set `/Game/ThirdPerson/Blueprints/BP_ThirdPersonCharacter.ObjetoInteractuable` null _asbp_third_person_character))

(event `/Game/Inventario/BPI_Interaccion.Interactuar`
  (bind _asbp_third_person_character (cast `/Game/ThirdPerson/Blueprints/BP_ThirdPersonCharacter` (`GameplayStatics.GetPlayerCharacter` 0)))
  (bind _output_get (set `self.Player` _asbp_third_person_character))
  (bind (_elemento _haylugar_) (`/Game/Inventario/BP_ControlInventario.Comprobar Hueco` (`/Game/ThirdPerson/Blueprints/BP_ThirdPersonCharacter.Inventario` _output_get)))
  (if _haylugar_
    (`/Game/Inventario/BP_ControlInventario.Cargar Objeto` (`/Game/ThirdPerson/Blueprints/BP_ThirdPersonCharacter.Inventario` (`self.Player`)) (`self.DatosObjeto`) _elemento)))

(fn `UserConstructionScript`)