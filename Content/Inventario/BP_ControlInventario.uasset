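; Inventory controller actor that registers itself on the third-person character at BeginPlay and manages an array of item data.
; ComprobarHueco finds the first empty slot by its image, and CargarObjeto stores an item there and destroys the character's interactable object.
; DescargarObjeto clears a slot and respawns the item's class at the character mesh, restoring its data.
; PintarInventario refreshes the HUD panel's slot widgets, showing frames only on filled slots.
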(event `self.ReceiveBeginPlay`
  (bind _asbp_third_person_character (cast `/Game/ThirdPerson/Blueprints/BP_ThirdPersonCharacter` (`GameplayStatics.GetPlayerCharacter` 0)))
  (set `/Game/ThirdPerson/Blueprints/BP_ThirdPersonCharacter.Inventario` self _asbp_third_person_character))

(fn `Cargar Objeto`
  (params (Item :type "/Game/Inventario/BPS_DatosEstructur Structure") (Posicion :type Integer))
  (locals (ItemCargado :type Integer) (PosicionCargada :type "/Game/Inventario/BPS_DatosEstructur Structure"))
  (set `local.PosicionCargada` Item)
  (bind _output_get (set `local.ItemCargado` Posicion))
  (if (`KismetMathLibrary.InRange_IntInt` _output_get 0 (`self.Tamano`))
    (`KismetArrayLibrary.Array_Set` (`self.DatosDelInevntario`) (`local.ItemCargado`) (`local.PosicionCargada`))
    (`self.K2_DestroyActor` (`/Game/ThirdPerson/Blueprints/BP_ThirdPersonCharacter.ObjetoInteractuable` (cast `/Game/ThirdPerson/Blueprints/BP_ThirdPersonCharacter` (`GameplayStatics.GetPlayerCharacter` 0) :!pure true)))))

(fn `Comprobar Hueco`
  (returns (Elemento :type Integer) (`HayLugar?` :type Boolean))
  (locals (`Elemento Vacio` :type Integer))
  (set `local.Elemento Vacio` -2)
  (for (_array_element _array_index) (`self.DatosDelInevntario`)
    (if (== (`.Imagen_17_22649F6B40D794CFB2B737A753A21882` (break `/Game/Inventario/BPS_DatosEstructur` _array_element)) null)
      (set `local.Elemento Vacio` _array_index)
      (break)))
  (if (== (`local.Elemento Vacio`) -2)
    (return (`local.Elemento Vacio`) false)
    (else
      (return (`local.Elemento Vacio`) true))))

(fn `Descargar Objeto`
  (params (Item :type "/Game/Inventario/BPS_DatosEstructur Structure") (Posicion :type Integer))
  (locals (ItemCargado :type "/Game/Inventario/BPS_DatosEstructur Structure"))
  (bind (_itemcargado_nombre _itemcargado_subnombre _itemcargado_descripcion _itemcargado_imagen _itemcargado_objeto _itemcargado_claseobjeto) (break `/Game/Inventario/BPS_DatosEstructur` (`local.ItemCargado`)))
  (bind (_itemcargado_nombre_2 _itemcargado_subnombre_2 _itemcargado_descripcion_2 _itemcargado_imagen_2 _itemcargado_objeto_2 _itemcargado_claseobjeto_2) (break `/Game/Inventario/BPS_DatosEstructur` (`local.ItemCargado`)))
  (set `local.ItemCargado` Item)
  (`KismetArrayLibrary.Array_Set` (`self.DatosDelInevntario`) Posicion)
  (bind _returnvalue (`|SpawnActorFromClass` _itemcargado_claseobjeto (`SceneComponent.K2_GetComponentToWorld` (`Character.Mesh` (cast `/Game/ThirdPerson/Blueprints/BP_ThirdPersonCharacter` (`GameplayStatics.GetPlayerCharacter` 0) :!pure true))) "Undefined" "MultiplyWithRoot" null null))
  (bind _asbp_objeto_interactuable (cast `/Game/Inventario/BP_ObjetoInteractuable` _returnvalue))
  (set `/Game/Inventario/BP_ObjetoInteractuable.DatosObjeto` (make `/Game/Inventario/BPS_DatosEstructur` _itemcargado_nombre_2 _itemcargado_subnombre_2 _itemcargado_descripcion_2 _itemcargado_imagen_2 _asbp_objeto_interactuable _itemcargado_claseobjeto_2) _asbp_objeto_interactuable))

(fn `Pintar Inventario`
  (locals (ContadorInventario :type Integer) (`Item Seleccionado` :type "/Game/Inventario/WBP_ItemUnico Object Reference") (Seleccionado :type "/Game/Inventario/BPS_DatosEstructur Structure"))
  (bind (_seleccionado_nombre _seleccionado_subnombre _seleccionado_descripcion _seleccionado_imagen) (break `/Game/Inventario/BPS_DatosEstructur` (`local.Seleccionado`)))
  (for (_array_element _array_index) (`self.DatosDelInevntario`)
    (set `local.Seleccionado` _array_element)
    (set `local.ContadorInventario` _array_index)
    (if (<= (`local.ContadorInventario`) (`self.Tamano`))
      (bind _aswbp_item_unico (cast `/Game/Inventario/WBP_ItemUnico` (`PanelWidget.GetChildAt` (`/Game/Inventario/HUD_Inventario.Panel` (`/Game/ThirdPerson/Blueprints/BP_ThirdPersonCharacter.RefInventarioHUD` (cast `/Game/ThirdPerson/Blueprints/BP_ThirdPersonCharacter` (`GameplayStatics.GetPlayerCharacter` 0) :!pure true))) (`local.ContadorInventario`))))
      (bind _output_get (set `local.Item Seleccionado` _aswbp_item_unico))
      (set `Widget.Visibility` "Visible" _output_get)
      (`Border.SetBrushFromTexture` (`/Game/Inventario/WBP_ItemUnico.Item` (`local.Item Seleccionado`)) _seleccionado_imagen)
      (if (== _seleccionado_imagen null)
        (`Border.SetBrushFromTexture` (`/Game/Inventario/WBP_ItemUnico.MArco` (`local.Item Seleccionado`)) "/Game/LevelPrototyping/Textures/T_GridChecker_A.T_GridChecker_A")
        (set `Widget.Visibility` "Hidden" (`/Game/Inventario/WBP_ItemUnico.MArco` (`local.Item Seleccionado`)))
        (else
          (`Border.SetBrushFromTexture` (`/Game/Inventario/WBP_ItemUnico.MArco` (`local.Item Seleccionado`)) "/Game/Characters/Mannequins/Textures/Shared/T_UE_Logo_M.T_UE_Logo_M")
          (set `Widget.Visibility` "Visible" (`/Game/Inventario/WBP_ItemUnico.MArco` (`local.Item Seleccionado`)))))
      (else
        (break)))))

(fn `UserConstructionScript`)